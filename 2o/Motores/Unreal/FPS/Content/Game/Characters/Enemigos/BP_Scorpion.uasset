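; BP_Scorpion is an enemy that chases pawns it sees and damages actors it touches.
; Its PawnSensing component triggers an AI MoveTo toward the seen pawn, stopping within an approach distance.
; A box collision overlap applies damage to any actor that is not another scorpion.
; Incoming damage lowers its Health, and the actor is destroyed when Health reaches zero or below.
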(event `self.ReceiveTick`
  (params (DeltaSeconds :type "Float (single-precision)")))

(event `self.ReceiveAnyDamage`
  (params (Damage :type "Float (single-precision)") (DamageType :type "DamageType Object Reference") (InstigatedBy :type "Controller Object Reference") (DamageCauser :type "Actor Object Reference"))
  (bind _health (`self.Health`))
  ;[1 1 1] Make & Take Damage
  (set `self.Health` (- _health Damage))
  (if (<= _health 0.0)
    (`self.K2_DestroyActor`)))

(event `self.BoxCollision.OnComponentBeginOverlap`
  (params (OverlappedComponent :type "PrimitiveComponent Object Reference") (OtherActor :type "Actor Object Reference") (OtherComp :type "PrimitiveComponent Object Reference") (OtherBodyIndex :type Integer) (bFromSweep :type Boolean) (SweepResult :type "HitResult Structure (by ref)"))
  ;[1 1 1] Make & Take Damage
  (if (not (`GameplayStatics.ObjectIsA` OtherActor "BP_Scorpion_C"))
    (`GameplayStatics.ApplyDamage` OtherActor (`self.Damage`))))

(event `self.PawnSensing.OnSeePawn`
  (params (Pawn :type "Pawn Object Reference"))
  (`|AIMoveTo` self (0.0 0.0 0.0) Pawn (`self.AproachDistance`) true))

(fn `UserConstructionScript`)