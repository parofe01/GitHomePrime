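; First-person player character with movement, look, jump, health that opens the lose menu at zero, and three guns: sniper, AK and revolver.
; BeginPlay spawns all three, and switching reattaches them between gun and hidden sockets; only Weapon1 skips the reload check.
; Shoot fires camera-based shots with delay-based fire rate and reload.
; A duplicate Shoot handler skips reload and sniper ammo checks, and revolver shots test the sniper's cooldown flag.
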(event `InputAxis|MoveUp`
  (params (AxisValue :type "Float (single-precision)"))
  ;[1 1 1] Movement & Camera
  (`self.AddMovementInput` (`self.GetActorForwardVector`) (* AxisValue (`self.Speed`))))

(event `InputAxis|LookUp`
  (params (AxisValue :type "Float (single-precision)"))
  ;[1 1 1] Movement & Camera
  (`self.AddControllerPitchInput` AxisValue))

(event `self.ReceiveBeginPlay`
  (bind _equippedgun1 (`self.EquippedGun1`))
  (bind _equippedgun3 (`self.EquippedGun3`))
  (bind _equippedgun2 (`self.EquippedGun2`))
  ;[1 1 1] SpawnArmas
  (bind _returnvalue (`|SpawnActorFromClass` "/Game/Game/Extras/BP_Sniper.BP_Sniper_C" (`KismetMathLibrary.MakeTransform` (0.0 0.0 0.0)) "Undefined" "MultiplyWithRoot" null null))
  (bind _output_get (set `self.EquippedGun1` _returnvalue))
  (`self.K2_AttachToComponent` _output_get (`self.GunLocation1`) "None" "SnapToTarget" "SnapToTarget" "KeepRelative" true)
  (set `/Game/Game/Extras/BP_BaseGun.Municion` (`/Game/Game/Extras/BP_BaseGun.MunicionMax` _equippedgun1) _equippedgun1)
  (bind _returnvalue_2 (`|SpawnActorFromClass` "/Game/Game/Extras/BP_AK.BP_AK_C" (`KismetMathLibrary.MakeTransform` (0.0 0.0 0.0)) "Undefined" "MultiplyWithRoot" null null))
  (bind _output_get_2 (set `self.EquippedGun2` _returnvalue_2))
  (`self.K2_AttachToComponent` _output_get_2 (`self.HiddenLocation2`) "None" "SnapToTarget" "SnapToTarget" "KeepRelative" true)
  (set `/Game/Game/Extras/BP_BaseGun.Municion` (`/Game/Game/Extras/BP_BaseGun.MunicionMax` _equippedgun2) _equippedgun2)
  (bind _returnvalue_3 (`|SpawnActorFromClass` "/Game/Game/Extras/BP_Revolver.BP_Revolver_C" (`KismetMathLibrary.MakeTransform` (0.0 0.0 0.0)) "Undefined" "MultiplyWithRoot" null null))
  (bind _output_get_3 (set `self.EquippedGun3` _returnvalue_3))
  (`self.K2_AttachToComponent` _output_get_3 (`self.HiddenLocation3`) "None" "SnapToTarget" "SnapToTarget" "KeepRelative" true)
  (set `/Game/Game/Extras/BP_BaseGun.Municion` (`/Game/Game/Extras/BP_BaseGun.MunicionMax` _equippedgun3) _equippedgun3))

(event `InputAxis|LookRight`
  (params (AxisValue :type "Float (single-precision)"))
  ;[1 1 1] Movement & Camera
  (`self.AddControllerYawInput` AxisValue))

(event `self.ReceiveAnyDamage`
  (params (Damage :type "Float (single-precision)") (DamageType :type "DamageType Object Reference") (InstigatedBy :type "Controller Object Reference") (DamageCauser :type "Actor Object Reference"))
  (bind _health (`self.Health`))
  ;[1 1 1] Take Damage
  (set `self.Health` (- _health Damage))
  (if (<= _health 0.0)
    (`GameplayStatics.OpenLevelBySoftObjectPtr` "/Game/Game/Levels/LoseMenu.LoseMenu")))

(event `InputAxis|MoveRight`
  (params (AxisValue :type "Float (single-precision)"))
  ;[1 1 1] Movement & Camera
  (`self.AddMovementInput` (`self.GetActorRightVector`) (* (`self.Speed`) AxisValue)))

(event `InputAction|Jump`
  (params (Key :type "Key Structure"))
  ;[1 1 1] Movement & Camera
  (:`Pressed`
    (`self.Jump`)))

(event `InputAction|Reload`
  (params (Key :type "Key Structure"))
  (bind _equippedgun1 (`self.EquippedGun1`))
  (bind _equippedgun3 (`self.EquippedGun3`))
  (bind _equippedgun2 (`self.EquippedGun2`))
  ;[1 1 1] Reload Switch
  (:`Pressed`
    (switch `int` (`self.WeaponSelected`)
      (:`0`
        ;[1 1 1] Reload Sniper
        (if (not (`/Game/Game/Extras/BP_BaseGun.Reloading` _equippedgun1))
          (set `/Game/Game/Extras/BP_BaseGun.Reloading` true _equippedgun1)
          (`KismetSystemLibrary.Delay` (`/Game/Game/Extras/BP_BaseGun.ReloadTime` _equippedgun1))
          (set `/Game/Game/Extras/BP_BaseGun.Municion` (`/Game/Game/Extras/BP_BaseGun.MunicionMax` _equippedgun1) _equippedgun1)
          (set `/Game/Game/Extras/BP_BaseGun.Reloading` false _equippedgun1)))
      (:`1`
        ;[1 1 1] Reload AK
        (if (not (`/Game/Game/Extras/BP_BaseGun.Reloading` _equippedgun2))
          (set `/Game/Game/Extras/BP_BaseGun.Reloading` true _equippedgun2)
          (`KismetSystemLibrary.Delay` (`/Game/Game/Extras/BP_BaseGun.ReloadTime` _equippedgun2))
          (set `/Game/Game/Extras/BP_BaseGun.Municion` (`/Game/Game/Extras/BP_BaseGun.MunicionMax` _equippedgun2) _equippedgun2)
          (set `/Game/Game/Extras/BP_BaseGun.Reloading` false _equippedgun2)))
      (:`2`
        ;[1 1 1] Reload Revolver
        (if (not (`/Game/Game/Extras/BP_BaseGun.Reloading` _equippedgun3))
          (set `/Game/Game/Extras/BP_BaseGun.Reloading` true _equippedgun3)
          (`KismetSystemLibrary.Delay` (`/Game/Game/Extras/BP_BaseGun.ReloadTime` _equippedgun3))
          (set `/Game/Game/Extras/BP_BaseGun.Municion` (`/Game/Game/Extras/BP_BaseGun.MunicionMax` _equippedgun3) _equippedgun3)
          (set `/Game/Game/Extras/BP_BaseGun.Reloading` false _equippedgun3))))))

(event `InputAction|Shoot`
  (params (Key :type "Key Structure"))
  (bind _fpscamera (`self.FPSCamera`))
  (bind _fpscamera_2 (`self.FPSCamera`))
  (bind _equippedgun1 (`self.EquippedGun1`))
  (bind _equippedgun3 (`self.EquippedGun3`))
  (bind _fpscamera_3 (`self.FPSCamera`))
  (bind _equippedgun2 (`self.EquippedGun2`))
  (bind _returnvalue (`SceneComponent.K2_GetComponentLocation` _fpscamera_3))
  (bind _returnvalue_2 (`SceneComponent.K2_GetComponentLocation` _fpscamera))
  (bind _returnvalue_3 (`SceneComponent.K2_GetComponentLocation` _fpscamera_2))
  (bind _municion (`/Game/Game/Extras/BP_BaseGun.Municion` _equippedgun3))
  (bind _municion_2 (`/Game/Game/Extras/BP_BaseGun.Municion` _equippedgun1))
  (bind _municion_3 (`/Game/Game/Extras/BP_BaseGun.Municion` _equippedgun2))
  ;[1 1 1] Shoot Switch
  (:`Pressed`
    (bind _returnvalue_4 (`self.ReloadingWeapon`))
    (if (not _returnvalue_4)
      (switch `int` (`self.WeaponSelected`)
        (:`0`
          ;[1 1 1] ShootSniper
          (if (and (`self.CanShoot1`) (>= _municion_2 1.0))
            (`/Game/Game/Extras/BP_BaseGun.Shoot` _equippedgun1 _returnvalue_3 (+ _returnvalue_3 (* (`/Game/Game/Extras/BP_BaseGun.MaxBulletDistance` _equippedgun1) (`SceneComponent.GetForwardVector` _fpscamera_2))))
            (`GameplayStatics.PlaySound2D` "/Game/Game/Sound/SND_shotgun-shoot-only.SND_shotgun-shoot-only" 1.0 1.0 0.0 null null)
            (set `/Game/Game/Extras/BP_BaseGun.Municion` (- _municion_2 1.0) _equippedgun1)
            (set `self.CanShoot1` false)
            (`KismetSystemLibrary.Delay` (`/Game/Game/Extras/BP_BaseGun.FireRate` _equippedgun1))
            (set `self.CanShoot1` true)))
        (:`1`
          ;[1 1 1] ShootAK
          (if (and (`self.CanShoot2`) (>= _municion_3 1.0))
            (`/Game/Game/Extras/BP_BaseGun.Shoot` _equippedgun2 _returnvalue (+ _returnvalue (* (`/Game/Game/Extras/BP_BaseGun.MaxBulletDistance` _equippedgun2) (`SceneComponent.GetForwardVector` _fpscamera_3))))
            (`GameplayStatics.PlaySound2D` "/Game/Game/Sound/SND_shotgun-shoot-only.SND_shotgun-shoot-only" 1.0 1.0 0.0 null null)
            (set `/Game/Game/Extras/BP_BaseGun.Municion` (- _municion_3 1.0) _equippedgun2)
            (set `self.CanShoot2` false)
            (`KismetSystemLibrary.Delay` (`/Game/Game/Extras/BP_BaseGun.FireRate` _equippedgun2))
            (set `self.CanShoot2` true)))
        (:`2`
          ;[1 1 1] ShootRevolver
          (if (and (`self.CanShoot1`) (>= _municion 1.0))
            (`/Game/Game/Extras/BP_BaseGun.Shoot` _equippedgun3 _returnvalue_2 (+ _returnvalue_2 (* (`/Game/Game/Extras/BP_BaseGun.MaxBulletDistance` _equippedgun3) (`SceneComponent.GetForwardVector` _fpscamera))))
            (`GameplayStatics.PlaySound2D` "/Game/Game/Sound/SND_shotgun-shoot-only.SND_shotgun-shoot-only" 1.0 1.0 0.0 null null)
            (set `/Game/Game/Extras/BP_BaseGun.Municion` (- _municion 1.0) _equippedgun3)
            (set `self.CanShoot3` false)
            (`KismetSystemLibrary.Delay` (`/Game/Game/Extras/BP_BaseGun.FireRate` _equippedgun3))
            (set `self.CanShoot3` true)))))))

(event `InputAction|Shoot`
  (params (Key :type "Key Structure"))
  (bind _fpscamera (`self.FPSCamera`))
  (bind _fpscamera_2 (`self.FPSCamera`))
  (bind _fpscamera_3 (`self.FPSCamera`))
  (bind _equippedgun2 (`self.EquippedGun2`))
  (bind _equippedgun1 (`self.EquippedGun1`))
  (bind _equippedgun3 (`self.EquippedGun3`))
  (bind _returnvalue (`SceneComponent.K2_GetComponentLocation` _fpscamera))
  (bind _returnvalue_2 (`SceneComponent.K2_GetComponentLocation` _fpscamera_2))
  (bind _returnvalue_3 (`SceneComponent.K2_GetComponentLocation` _fpscamera_3))
  (bind _municion (`/Game/Game/Extras/BP_BaseGun.Municion` _equippedgun3))
  (bind _municion_2 (`/Game/Game/Extras/BP_BaseGun.Municion` _equippedgun2))
  ;[1 1 1] Shoot Switch
  (:`Pressed`
    (switch `int` (`self.WeaponSelected`)
      (:`0`
        ;[1 1 1] ShootSniper
        (if (`self.CanShoot1`)
          (`/Game/Game/Extras/BP_BaseGun.Shoot` _equippedgun1 _returnvalue_2 (+ _returnvalue_2 (* (`/Game/Game/Extras/BP_BaseGun.MaxBulletDistance` _equippedgun1) (`SceneComponent.GetForwardVector` _fpscamera_2))))
          (`GameplayStatics.PlaySound2D` "/Game/Game/Sound/SND_shotgun-shoot-only.SND_shotgun-shoot-only" 1.0 1.0 0.0 null null)
          (set `self.CanShoot1` false)
          (`KismetSystemLibrary.Delay` (`/Game/Game/Extras/BP_BaseGun.FireRate` _equippedgun1))
          (set `self.CanShoot1` true)))
      (:`1`
        ;[1 1 1] ShootAK
        (if (and (`self.CanShoot2`) (>= _municion_2 1.0))
          (`/Game/Game/Extras/BP_BaseGun.Shoot` _equippedgun2 _returnvalue_3 (+ _returnvalue_3 (* (`/Game/Game/Extras/BP_BaseGun.MaxBulletDistance` _equippedgun2) (`SceneComponent.GetForwardVector` _fpscamera_3))))
          (`GameplayStatics.PlaySound2D` "/Game/Game/Sound/SND_shotgun-shoot-only.SND_shotgun-shoot-only" 1.0 1.0 0.0 null null)
          (set `/Game/Game/Extras/BP_BaseGun.Municion` (- _municion_2 1.0) _equippedgun2)
          (set `self.CanShoot2` false)
          (`KismetSystemLibrary.Delay` (`/Game/Game/Extras/BP_BaseGun.FireRate` _equippedgun2))
          (set `self.CanShoot2` true)))
      (:`2`
        ;[1 1 1] ShootRevolver
        (if (and (`self.CanShoot1`) (>= _municion 1.0))
          (`/Game/Game/Extras/BP_BaseGun.Shoot` _equippedgun3 _returnvalue (+ _returnvalue (* (`/Game/Game/Extras/BP_BaseGun.MaxBulletDistance` _equippedgun3) (`SceneComponent.GetForwardVector` _fpscamera))))
          (`GameplayStatics.PlaySound2D` "/Game/Game/Sound/SND_shotgun-shoot-only.SND_shotgun-shoot-only" 1.0 1.0 0.0 null null)
          (set `/Game/Game/Extras/BP_BaseGun.Municion` (- _municion 1.0) _equippedgun3)
          (set `self.CanShoot3` false)
          (`KismetSystemLibrary.Delay` (`/Game/Game/Extras/BP_BaseGun.FireRate` _equippedgun3))
          (set `self.CanShoot3` true))))))

(event `InputAction|Weapon1`
  (params (Key :type "Key Structure"))
  ;[1 1 1] WeaponSwitch
  (:`Pressed`
    (set `self.WeaponSelected` 0)
    (`self.K2_AttachToComponent` (`self.EquippedGun1`) (`self.GunLocation1`) "None" "SnapToTarget" "SnapToTarget" "KeepRelative" true)
    (`self.K2_AttachToComponent` (`self.EquippedGun2`) (`self.HiddenLocation2`) "None" "SnapToTarget" "SnapToTarget" "KeepRelative" true)
    (`self.K2_AttachToComponent` (`self.EquippedGun3`) (`self.HiddenLocation3`) "None" "SnapToTarget" "SnapToTarget" "KeepRelative" true)))

(event `InputAction|Weapon2`
  (params (Key :type "Key Structure"))
  ;[1 1 1] WeaponSwitch
  (:`Pressed`
    (bind _returnvalue (`self.ReloadingWeapon`))
    (if (not _returnvalue)
      (set `self.WeaponSelected` 1)
      (`self.K2_AttachToComponent` (`self.EquippedGun1`) (`self.HidenLocation1`) "None" "SnapToTarget" "SnapToTarget" "KeepRelative" true)
      (`self.K2_AttachToComponent` (`self.EquippedGun2`) (`self.GunLocation2`) "None" "SnapToTarget" "SnapToTarget" "KeepRelative" true)
      (`self.K2_AttachToComponent` (`self.EquippedGun3`) (`self.HiddenLocation3`) "None" "SnapToTarget" "SnapToTarget" "KeepRelative" true))))

(event `InputAction|Weapon3`
  (params (Key :type "Key Structure"))
  ;[1 1 1] WeaponSwitch
  (:`Pressed`
    (bind _returnvalue (`self.ReloadingWeapon`))
    (if (not _returnvalue)
      (set `self.WeaponSelected` 2)
      (`self.K2_AttachToComponent` (`self.EquippedGun1`) (`self.HidenLocation1`) "None" "SnapToTarget" "SnapToTarget" "KeepRelative" true)
      (`self.K2_AttachToComponent` (`self.EquippedGun2`) (`self.HiddenLocation2`) "None" "SnapToTarget" "SnapToTarget" "KeepRelative" true)
      (`self.K2_AttachToComponent` (`self.EquippedGun3`) (`self.GunLocation3`) "None" "SnapToTarget" "SnapToTarget" "KeepRelative" true))))

(fn `ReloadingWeapon`
  (returns (ReturnValue :type Boolean))
  (return (or (`/Game/Game/Extras/BP_BaseGun.Reloading` (`self.EquippedGun1`)) (`/Game/Game/Extras/BP_BaseGun.Reloading` (`self.EquippedGun2`)) (`/Game/Game/Extras/BP_BaseGun.Reloading` (`self.EquippedGun3`)))))

(fn `UserConstructionScript`)