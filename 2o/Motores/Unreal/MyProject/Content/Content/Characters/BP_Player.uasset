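; BP_Player is the player character, with axis-driven movement and camera look, jumping and a hitscan shot.
; Shooting line-traces from the camera with persistent debug drawing, spawns an explosion at any hit and calls TakeDamage on a hit BP_Enemy.
; BeginPlay adds the BP_UI widget to the viewport, and AnyDamage subtracts from Health with no death handling.
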(event `InputAxis|MovimientoForward`
  (params (AxisValue :type "Float (single-precision)"))
  ;[0.3229 1 0.3229] Movement
  (`self.AddMovementInput` (`self.GetActorForwardVector`) (* AxisValue (`self.Speed`))))

(event `InputAxis|CameraUp`
  (params (AxisValue :type "Float (single-precision)"))
  ;[0.3229 1 0.3229] Movement
  (`self.AddControllerPitchInput` AxisValue))

(event `InputAxis|CameraRight`
  (params (AxisValue :type "Float (single-precision)"))
  ;[0.3229 1 0.3229] Movement
  (`self.AddControllerYawInput` AxisValue))

(event `InputAxis|MovimientoRight`
  (params (AxisValue :type "Float (single-precision)"))
  ;[0.3229 1 0.3229] Movement
  (`self.AddMovementInput` (`self.GetActorRightVector`) (* (`self.Speed`) AxisValue)))

(event `InputAction|Jump`
  (params (Key :type "Key Structure"))
  ;[0.3229 1 0.3229] Movement
  (:`Pressed`
    (`self.Jump`)))

(event `InputAction|Shoot`
  (params (Key :type "Key Structure"))
  (bind _camera (`self.Camera`))
  (bind _returnvalue (`SceneComponent.K2_GetComponentLocation` _camera))
  ;[1 0.3333 0.3333] Shoot
  (:`Pressed`
    (bind (_outhit _returnvalue_2) (`KismetSystemLibrary.LineTraceSingle` :`Start` _returnvalue :`End` (+ _returnvalue (* (`SceneComponent.GetForwardVector` _camera) (`self.MaxDistance`))) :`TraceChannel` "TraceTypeQuery3" :`DrawDebugType` "Persistent"))
    (if _returnvalue_2
      (`GameplayStatics.SpawnEmitterAtLocation` "/Game/StarterContent/Particles/P_Explosion.P_Explosion" (`.Location` (`GameplayStatics.BreakHitResult` _outhit)))
      (if (`GameplayStatics.ObjectIsA` (`.HitActor` (`GameplayStatics.BreakHitResult` _outhit)) "/Game/Content/Characters/BP_Enemy.BP_Enemy_C")
        (`KismetSystemLibrary.PrintString` "Hello")
        (bind _asbp_enemy (cast `/Game/Content/Characters/BP_Enemy` (`.HitActor` (`GameplayStatics.BreakHitResult` _outhit))))
        (`/Game/Content/Characters/BP_Enemy.TakeDamage` _asbp_enemy)))))

(event `self.ReceiveBeginPlay`
  ;[0.4059 0.9801 1] Take Damage
  (bind _returnvalue (`|CreateWidget` "/Game/Content/UI/BP_UI.BP_UI_C"))
  (`UserWidget.AddToViewport` _returnvalue 0))

(event `self.ReceiveAnyDamage`
  (params (Damage :type "Float (single-precision)") (DamageType :type "DamageType Object Reference") (InstigatedBy :type "Controller Object Reference") (DamageCauser :type "Actor Object Reference"))
  ;[0.4059 0.9801 1] Take Damage
  (set `self.Health` (- (`self.Health`) Damage)))

(fn `UserConstructionScript`)